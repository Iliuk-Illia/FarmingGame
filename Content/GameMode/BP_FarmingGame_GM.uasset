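; Game mode for the farming game that persists per-level changes to placed and removed actors across sessions.
; On BeginPlay or Continue, it loads or creates a SaveData_Level save keyed by level name and the game instance's slot index.
; Loading respawns added actors by transform, restores Plant growth, bush and inventory-origin flags, then destroys actors recorded as removed.
; EndPlay writes the level save back to its slot.
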(event Custom|Continue
  (bind _asfarming_game_instance (Utilities|Casting|CastToFarmingGameInstance (Game|GetGameInstance)))
  (bind _returnvalue (Game|GetCurrentLevelName true))
  (bind _output_get (Variables|Default|SetSlot%20Name (Utilities|String|Append (Utilities|String|Append _returnvalue "_Data") (Utilities|String|ToString(Integer) (Variables|/Script/FarmingGame.FarmingGameInstance|GetSlotIndex _asfarming_game_instance)))))
  (bind _returnvalue_2 (SaveGame|DoesSaveGameExist _output_get))
  (if _returnvalue_2
    (bind _returnvalue_3 (SaveGame|LoadGamefromSlot (Variables|Default|GetSlot%20Name)))
    (bind _assave_data_level (Utilities|Casting|CastToSaveData_Level _returnvalue_3))
    (bind _output_get_2 (Variables|Default|SetAs%20Save%20Data%20Level _assave_data_level))
    (SaveGame|SaveGametoSlot _output_get_2 (Variables|Default|GetSlot%20Name))
    (bind _keys (Utilities|Map|Keys (Variables|/Game/GameMode/SaveData_Level.SaveData_Level_C|GetActorsAdded (Variables|Default|GetAs%20Save%20Data%20Level))))
    (for _array_element _keys
      (bind _returnvalue_4 (Game|SpawnActorfromClass (Utilities|ResolveSoftReference (.Value (Utilities|Map|Find (Variables|/Game/GameMode/SaveData_Level.SaveData_Level_C|GetActorsAdded (Variables|Default|GetAs%20Save%20Data%20Level)) _array_element))) _array_element "AlwaysSpawn" "MultiplyWithRoot" 0 0))
      (bind _asplant (Utilities|Casting|CastToPlant _returnvalue_4))
      (Variables|/Script/FarmingGame.ItemDataComponent|SetIsFullyGrown (Variables|/Game/Inventory/Plants/Plant.Plant_C|GetItemData _asplant) (.full (.Value (Utilities|Map|Find (Variables|/Game/GameMode/SaveData_Level.SaveData_Level_C|GetActorsInfo (Variables|Default|GetAs%20Save%20Data%20Level)) _array_element))))
      (Variables|/Script/FarmingGame.ItemDataComponent|SetIsBush (Variables|/Game/Inventory/Plants/Plant.Plant_C|GetItemData _asplant) (.bush (.Value (Utilities|Map|Find (Variables|/Game/GameMode/SaveData_Level.SaveData_Level_C|GetActorsInfo (Variables|Default|GetAs%20Save%20Data%20Level)) _array_element))))
      (Variables|/Script/FarmingGame.CppPlant|SetFromInventory _asplant (.frominventory (.Value (Utilities|Map|Find (Variables|/Game/GameMode/SaveData_Level.SaveData_Level_C|GetActorsInfo (Variables|Default|GetAs%20Save%20Data%20Level)) _array_element)))))
    (for _array_element_2 (Variables|/Game/GameMode/SaveData_Level.SaveData_Level_C|GetActorsRemoved (Variables|Default|GetAs%20Save%20Data%20Level))
      (Utilities|IsValid (Utilities|ResolveSoftReference _array_element_2)
        (:Is%20Valid
          (Actor|DestroyActor (Utilities|ResolveSoftReference _array_element_2)))))
    (else
      (bind _returnvalue_5 (SaveGame|CreateSaveGameObject "/Game/GameMode/SaveData_Level.SaveData_Level_C"))
      (bind _output_get_3 (Variables|Default|SetAs%20Save%20Data%20Level _returnvalue_5))
      (SaveGame|SaveGametoSlot _output_get_3 (Variables|Default|GetSlot%20Name)))))

(event EventBeginPlay
  (bind _asfarming_game_instance (Utilities|Casting|CastToFarmingGameInstance (Game|GetGameInstance)))
  (bind _returnvalue (Game|GetCurrentLevelName true))
  (bind _output_get (Variables|Default|SetSlot%20Name (Utilities|String|Append (Utilities|String|Append _returnvalue "_Data") (Utilities|String|ToString(Integer) (Variables|/Script/FarmingGame.FarmingGameInstance|GetSlotIndex _asfarming_game_instance)))))
  (bind _returnvalue_2 (SaveGame|DoesSaveGameExist _output_get))
  (if _returnvalue_2
    (bind _returnvalue_3 (SaveGame|LoadGamefromSlot (Variables|Default|GetSlot%20Name)))
    (bind _assave_data_level (Utilities|Casting|CastToSaveData_Level _returnvalue_3))
    (bind _output_get_2 (Variables|Default|SetAs%20Save%20Data%20Level _assave_data_level))
    (SaveGame|SaveGametoSlot _output_get_2 (Variables|Default|GetSlot%20Name))
    (bind _keys (Utilities|Map|Keys (Variables|/Game/GameMode/SaveData_Level.SaveData_Level_C|GetActorsAdded (Variables|Default|GetAs%20Save%20Data%20Level))))
    (for _array_element _keys
      (bind _returnvalue_4 (Game|SpawnActorfromClass (Utilities|ResolveSoftReference (.Value (Utilities|Map|Find (Variables|/Game/GameMode/SaveData_Level.SaveData_Level_C|GetActorsAdded (Variables|Default|GetAs%20Save%20Data%20Level)) _array_element))) _array_element "AlwaysSpawn" "MultiplyWithRoot" 0 0))
      (bind _asplant (Utilities|Casting|CastToPlant _returnvalue_4))
      (Variables|/Script/FarmingGame.ItemDataComponent|SetIsFullyGrown (Variables|/Game/Inventory/Plants/Plant.Plant_C|GetItemData _asplant) (.full (.Value (Utilities|Map|Find (Variables|/Game/GameMode/SaveData_Level.SaveData_Level_C|GetActorsInfo (Variables|Default|GetAs%20Save%20Data%20Level)) _array_element))))
      (Variables|/Script/FarmingGame.ItemDataComponent|SetIsBush (Variables|/Game/Inventory/Plants/Plant.Plant_C|GetItemData _asplant) (.bush (.Value (Utilities|Map|Find (Variables|/Game/GameMode/SaveData_Level.SaveData_Level_C|GetActorsInfo (Variables|Default|GetAs%20Save%20Data%20Level)) _array_element))))
      (Variables|/Script/FarmingGame.CppPlant|SetFromInventory _asplant (.frominventory (.Value (Utilities|Map|Find (Variables|/Game/GameMode/SaveData_Level.SaveData_Level_C|GetActorsInfo (Variables|Default|GetAs%20Save%20Data%20Level)) _array_element)))))
    (for _array_element_2 (Variables|/Game/GameMode/SaveData_Level.SaveData_Level_C|GetActorsRemoved (Variables|Default|GetAs%20Save%20Data%20Level))
      (Utilities|IsValid (Utilities|ResolveSoftReference _array_element_2)
        (:Is%20Valid
          (Actor|DestroyActor (Utilities|ResolveSoftReference _array_element_2)))))
    (else
      (bind _returnvalue_5 (SaveGame|CreateSaveGameObject "/Game/GameMode/SaveData_Level.SaveData_Level_C"))
      (bind _output_get_3 (Variables|Default|SetAs%20Save%20Data%20Level _returnvalue_5))
      (SaveGame|SaveGametoSlot _output_get_3 (Variables|Default|GetSlot%20Name)))))

(event EventEndPlay
  (params (EndPlayReason :type EEndPlayReason%20Enum :default "Destroyed"))
  (SaveGame|SaveGametoSlot (Variables|Default|GetAs%20Save%20Data%20Level) (Variables|Default|GetSlot%20Name)))

(fn ConstructionScript)