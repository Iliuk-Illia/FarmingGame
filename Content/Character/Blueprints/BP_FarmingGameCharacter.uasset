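; First-person player character for a farming game that plants seeds and removes plants.
; BeginPlay creates the message widget for the Inventory and the Hotbar; Escape pauses into a menu.
; Left click traces from the camera to a box component, spawns the hotbar seed's data-table class there and consumes it from the Inventory.
; K traces to destroy a Plant, key 1 calls an inventory debug function, and both traces leave debug drawing on.
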(event EventBeginPlay
  (bind _returnvalue (UserInterface|CreateWidget "/Game/Inventory/UI/W_DisplayMessage.W_DisplayMessage_C"))
  (bind _output_get (Variables|/Script/FarmingGame.InventorySystem|SetMessageWidget (Variables|Default|GetInventory) _returnvalue))
  (UserInterface|Viewport|AddtoViewport _output_get 0)
  (bind _returnvalue_2 (UserInterface|CreateWidget "/Game/Inventory/UI/W_Hotbar.W_Hotbar_C"))
  (bind _output_get_2 (Variables|Default|SetHotbar _returnvalue_2))
  (UserInterface|Viewport|AddtoViewport _output_get_2 1))

(event Input|KeyboardEvents|1
  (params (Key :type Key%20Structure :default "None"))
  (:Pressed
    (Class|InventorySystem|DebugFunction (Variables|Default|GetInventory))))

(event Input|KeyboardEvents|Escape
  (params (Key :type Key%20Structure :default "None"))
  (bind _returnvalue (Game|GetPlayerController 0))
  (:Pressed
    (Game|SetGamePaused true)
    (bind _returnvalue_2 (UserInterface|CreateWidget "/Game/Inventory/UI/Menu/W_PauseMenu.W_PauseMenu_C"))
    (UserInterface|Viewport|AddtoViewport _returnvalue_2 0)
    (Variables|/Script/Engine.PlayerController|SetbShowMouseCursor _returnvalue true)
    (Input|SetInputModeUIOnly _returnvalue _returnvalue_2 "DoNotLock" false)))

(event Input|MouseEvents|LeftMouseButton
  (params (Key :type Key%20Structure :default "None"))
  (bind _firstpersoncameracomponent (Variables|Default|GetFirstPersonCameraComponent))
  (bind _hotbar (Variables|Default|GetHotbar))
  (bind _returnvalue (Transformation|GetWorldLocation _firstpersoncameracomponent))
  (bind _w_hotbarslot (Variables|/Game/Inventory/UI/W_Hotbar.W_Hotbar_C|GetW_HotbarSlot _hotbar))
  (bind _itemid (Variables|/Game/Inventory/UI/W_HotbarSlot.W_HotbarSlot_C|GetItemID _w_hotbarslot))
  (:Pressed
    (bind _outhit (Collision|LineTraceByChannel _returnvalue (+ _returnvalue (* (Math|Vector|GetForwardVector (Transformation|GetWorldRotation _firstpersoncameracomponent)) 2e+02)) "TraceTypeQuery1" false (Utilities|Array|MakeArray self) "ForDuration"))
    (if (.bBlockingHit (Collision|BreakHitResult _outhit))
      (Development|PrintString "Hello")
      (Utilities|Casting|CastToBoxComponent (.HitComponent (Collision|BreakHitResult _outhit)))
      (if (Utilities|String|Contains (Utilities|String|ToString(Name) _itemid) "Seed")
        (bind _returnvalue_2 (Utilities|GetDataTableRow "/Game/Inventory/NewDataTable.NewDataTable" _itemid)
          (:then
            (bind _returnvalue_3 (Game|SpawnActorfromClass (.ItemClass (Utilities|Struct|BreakItemStruct _returnvalue_2)) (Math|Transform|MakeTransform (.location (Transformation|GetWorldTransform (.HitComponent (Collision|BreakHitResult _outhit)))) (.rotation (Transformation|GetWorldTransform (.HitComponent (Collision|BreakHitResult _outhit))))) "AdjustIfPossibleButAlwaysSpawn" "MultiplyWithRoot" 0 0))
            (Class|IGrowInterface|Growing(Message) _returnvalue_3)
            (Class|InventorySystem|RemovefromInventory (Variables|Default|GetInventory) (Variables|/Game/Inventory/UI/W_HotbarSlot.W_HotbarSlot_C|GetInventoryIndex _w_hotbarslot) false true)))))))

(event Input|KeyboardEvents|K
  (params (Key :type Key%20Structure :default "None"))
  (bind _firstpersoncameracomponent (Variables|Default|GetFirstPersonCameraComponent))
  (bind _returnvalue (Transformation|GetWorldLocation _firstpersoncameracomponent))
  (:Pressed
    (bind (_outhit _returnvalue_2) (Collision|LineTraceByChannel _returnvalue (+ _returnvalue (* (Math|Vector|GetForwardVector (Transformation|GetWorldRotation _firstpersoncameracomponent)) 3e+02)) "TraceTypeQuery1" false (Utilities|Array|MakeArray self) "ForDuration"))
    (if _returnvalue_2
      (bind _asplant (Utilities|Casting|CastToPlant (.HitActor (Collision|BreakHitResult _outhit))))
      (Actor|DestroyActor _asplant))))

(fn ConstructionScript)