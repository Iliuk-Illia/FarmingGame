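; BP_InventorySystem holds inventory contents and saves and loads them for non-character inventories such as containers.
; Save and load events reach the level save data through BP_FarmingGame_GM, writing or reading Content in its ContainersAdded map.
; Each map entry is a container struct keyed by the inventory object itself.
; BeginPlay and Tick are unused, so both events run only when called.
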(event EventBeginPlay)

(event EventTick
  (params (DeltaSeconds :type Float%20%28single-precision%29)))

(event EventLoadInventoryNotCharacter
  (bind _asbp_farming_game_gm (Utilities|Casting|CastToBP_FarmingGame_GM (Game|GetGameMode)))
  (Variables|Default|SetContent (.Contents (Utilities|Struct|BreakFContainerStruct (.Value (Utilities|Map|Find (Variables|/Game/GameMode/SaveData_Level.SaveData_Level_C|GetContainersAdded (Variables|/Game/GameMode/BP_FarmingGame_GM.BP_FarmingGame_GM_C|GetAs%20Save%20Data%20Level _asbp_farming_game_gm)) (Utilities|ResolveSoftReference self)))))))

(event EventSaveInventoryNotCharacter
  (bind _asbp_farming_game_gm (Utilities|Casting|CastToBP_FarmingGame_GM (Game|GetGameMode)))
  (Utilities|Map|Add (Variables|/Game/GameMode/SaveData_Level.SaveData_Level_C|GetContainersAdded (Variables|/Game/GameMode/BP_FarmingGame_GM.BP_FarmingGame_GM_C|GetAs%20Save%20Data%20Level _asbp_farming_game_gm)) (Utilities|ResolveSoftReference self) (Utilities|Struct|MakeFContainerStruct (Variables|Default|GetContent) "0.000000,0.000000,0.000000|0.000000,0.000000,0.000000|1.000000,1.000000,1.000000")))